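; BP_Door is a key-locked puzzle door that opens when the game mode's current key matches its key number.
; BeginPlay caches the InGameMode, and Interact compares its CurrentKey to Keynumber, printing a message on a mismatch.
; On a match, the Door_rotate timeline slides the door mesh between start and end relative positions, despite its name.
; The construction script applies a per-instance material to the door.
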(event `self.ReceiveBeginPlay`
  ;[0.6732 1 0.3186] BP_Door eventgraph
  (bind _asin_game_mode (cast `/Game/PuzzleGame/midterm/InGameMode` (`GameplayStatics.GetGameMode`)))
  (set `self.As in Game Mode` _asin_game_mode))

(event `/Game/PuzzleGame/midterm/BPI_Maze.Interact`
  ;[0.6732 1 0.3186] BP_Door eventgraph
  (if (== (`/Game/PuzzleGame/midterm/InGameMode.CurrentKey` (`self.As in Game Mode`)) (`self.keynumber`))
    (bind (_direction _newtrack_1) (`Timeline|door_rotate`)
      (:`Update`
        (`SceneComponent.K2_SetRelativeLocation` (`self.door`) (`KismetMathLibrary.VLerp` (`self.startposiiton`) (`self.endposiiton`) _newtrack_1) false false)))
    (else
      (`KismetSystemLibrary.PrintString` "you dont have right key moron!"))))

(fn `UserConstructionScript`
  ;[0.1464 0.5356 1] bp_door construiction / aynı seyi key icin de yapcan
  (`PrimitiveComponent.SetMaterial` (`self.door`) 0 (`self.Material`)))