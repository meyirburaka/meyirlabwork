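; Spawner actor for the puzzle game that places a single Gascloud hazard at a random spot when play begins.
; BeginPlay rolls random X and Y multipliers, scales them into offsets from the spawner's location, and spawns the cloud there with the spawner's height and rotation, ignoring collision.
; Similar spawn nodes for BP_Axe and BP_spike are present but disconnected, so they never run.
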(event `self.ReceiveBeginPlay`
  (bind _returnvalue (`self.GetTransform`))
  (set `self.max x` (`KismetMathLibrary.RandomFloatInRange` 0.0 6.0))
  (set `self.max Y` (`KismetMathLibrary.RandomFloatInRange` 0.0 6.0))
  (`|ExecutionSequence`
    (:`then_1`
      (`|SpawnActorFromClass` "/Game/PuzzleGame/midterm/trapler/gascloud.gascloud_C" (`KismetMathLibrary.MakeTransform` (`KismetMathLibrary.MakeVector` (+ (* (`self.max x`) 500.0) (.x (.location _returnvalue))) (+ (* (`self.max Y`) 500.0) (.y (.location _returnvalue))) (.z (.location _returnvalue))) (.rotation _returnvalue)) "AlwaysSpawn" "MultiplyWithRoot" null null))))

(fn `UserConstructionScript`)