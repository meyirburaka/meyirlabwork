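; BP_axetrap is a swinging axe trap for a puzzle game, with an active state triggered by breaking its ropes.
; Eventrope sets IsAxeactive and destroys the four rope components.
; Axemove drives a pendulum swing by setting AxeRoot's roll from a sine of Time, 45 degrees either side of 180.
; The event graph holds only disabled stubs, and neither function is called within this Blueprint.
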(fn `axemove`
  (bind _axeroot (`self.AxeRoot`))
  (bind (_relativerotation_roll _relativerotation_pitch _relativerotation_yaw) (`KismetMathLibrary.BreakRotator` (`SceneComponent.RelativeRotation` _axeroot)))
  (bind _output_get (set `self.sinvalue` (* (`KismetMathLibrary.DegSin` (* (`self.Time`) 360.0)) 45.0)))
  (`SceneComponent.K2_SetRelativeRotation` _axeroot (`KismetMathLibrary.MakeRotator` (+ _output_get 180.0) _relativerotation_pitch _relativerotation_yaw) false false))

(fn `eventrope`
  (set `self.isAxeactive` true)
  (`ActorComponent.K2_DestroyComponent` (`self.Rope4`))
  (`ActorComponent.K2_DestroyComponent` (`self.Rope3`))
  (`ActorComponent.K2_DestroyComponent` (`self.Rope2`))
  (`ActorComponent.K2_DestroyComponent` (`self.Rope1`)))

(fn `UserConstructionScript`
  (`parent.UserConstructionScript`))