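; BP_Axe is a swinging axe trap that stays idle until one of its four rope triggers is overlapped.
; Any rope overlap activates the axe and destroys all four ropes.
; While active, Tick accumulates time to drive a sine-wave roll on AxeRoot, producing a pendulum swing.
; Any overlap on the We component calls Damageaxe on the player character cached at BeginPlay, without checking the overlapping actor.
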(event `self.ReceiveBeginPlay`
  (bind _asbp_third_person_character (cast `/Game/ThirdPerson/Blueprints/BP_ThirdPersonCharacter` (`GameplayStatics.GetPlayerPawn` 0)))
  (set `self.As BP Third Person Character` _asbp_third_person_character))

(event `self.ReceiveTick`
  (params (DeltaSeconds :type "Float (single-precision)"))
  (if (`self.isAxeactive`)
    (set `self.Time` (+ DeltaSeconds (`self.Time`)))
    (`self.axemove`)))

(event `self.Rope3.OnComponentBeginOverlap`
  (params (OverlappedComponent :type "PrimitiveComponent Object Reference") (OtherActor :type "Actor Object Reference") (OtherComp :type "PrimitiveComponent Object Reference") (OtherBodyIndex :type Integer) (bFromSweep :type Boolean) (SweepResult :type "HitResult Structure (by ref)"))
  (`self.eventrope` :!label _label))

(event `self.Rope1.OnComponentBeginOverlap`
  (params (OverlappedComponent :type "PrimitiveComponent Object Reference") (OtherActor :type "Actor Object Reference") (OtherComp :type "PrimitiveComponent Object Reference") (OtherBodyIndex :type Integer) (bFromSweep :type Boolean) (SweepResult :type "HitResult Structure (by ref)"))
  (goto _label))

(event `self.Rope4.OnComponentBeginOverlap`
  (params (OverlappedComponent :type "PrimitiveComponent Object Reference") (OtherActor :type "Actor Object Reference") (OtherComp :type "PrimitiveComponent Object Reference") (OtherBodyIndex :type Integer) (bFromSweep :type Boolean) (SweepResult :type "HitResult Structure (by ref)"))
  (goto _label))

(event `self.Rope2.OnComponentBeginOverlap`
  (params (OverlappedComponent :type "PrimitiveComponent Object Reference") (OtherActor :type "Actor Object Reference") (OtherComp :type "PrimitiveComponent Object Reference") (OtherBodyIndex :type Integer) (bFromSweep :type Boolean) (SweepResult :type "HitResult Structure (by ref)"))
  (goto _label))

(event `self.we.OnComponentBeginOverlap`
  (params (OverlappedComponent :type "PrimitiveComponent Object Reference") (OtherActor :type "Actor Object Reference") (OtherComp :type "PrimitiveComponent Object Reference") (OtherBodyIndex :type Integer) (bFromSweep :type Boolean) (SweepResult :type "HitResult Structure (by ref)"))
  (`/Game/ThirdPerson/Blueprints/BP_ThirdPersonCharacter.damageaxe` (`self.As BP Third Person Character`)))

(fn `axemove`
  (bind _axeroot (`self.AxeRoot`))
  (bind (_relativerotation_roll _relativerotation_pitch _relativerotation_yaw) (`KismetMathLibrary.BreakRotator` (`SceneComponent.RelativeRotation` _axeroot)))
  (bind _output_get (set `self.Sinvalue` (* (`KismetMathLibrary.DegSin` (* (`self.Time`) 360.0)) 45.0)))
  (`SceneComponent.K2_SetRelativeRotation` _axeroot (`KismetMathLibrary.MakeRotator` (+ _output_get 180.0) _relativerotation_pitch _relativerotation_yaw) false false))

(fn `eventrope`
  (set `self.isAxeactive` true)
  (`ActorComponent.K2_DestroyComponent` (`self.Rope4`))
  (`ActorComponent.K2_DestroyComponent` (`self.Rope3`))
  (`ActorComponent.K2_DestroyComponent` (`self.Rope2`))
  (`ActorComponent.K2_DestroyComponent` (`self.Rope1`)))

(fn `UserConstructionScript`)