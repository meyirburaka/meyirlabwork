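; BP_GasKEY_3 is an interactable key pickup in the midterm puzzle game.
; BeginPlay caches the InGameMode and the BP_ThirdPersonCharacter pawn, though the game mode reference is not used in these graphs.
; Interact clears the character's Axevurur flag and destroys the key actor.
; The construction script applies the Material variable to the Key component's first material slot.
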(event `self.ReceiveBeginPlay`
  ;[1 0.1781 0.1781] BP_Key eventgraph
  (bind _asin_game_mode (cast `/Game/PuzzleGame/midterm/InGameMode` (`GameplayStatics.GetGameMode`)))
  (set `self.As in Game Mode` _asin_game_mode)
  (bind _asbp_third_person_character (cast `/Game/ThirdPerson/Blueprints/BP_ThirdPersonCharacter` (`GameplayStatics.GetPlayerPawn` 0))))

(event `self.Interact`
  ;[1 0.1781 0.1781] BP_Key eventgraph
  (set `/Game/ThirdPerson/Blueprints/BP_ThirdPersonCharacter.axevurur` false (stale `self.ReceiveBeginPlay` _asbp_third_person_character))
  (`self.K2_DestroyActor`))

(fn `UserConstructionScript`
  (`PrimitiveComponent.SetMaterial` (`self.Key`) 0 (`self.Material`)))