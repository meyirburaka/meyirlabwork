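; BP_spike is a one-shot spike trap that damages the player when its pressure plate is overlapped.
; BeginPlay caches the player pawn as BP_ThirdPersonCharacter.
; The first Plate overlap by anything passes a DoOnce, calls Damagespike on that cached character and sets nine spike components to full scale.
; After a short delay the actor destroys itself.
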(event `self.ReceiveBeginPlay`
  (bind _asbp_third_person_character (cast `/Game/ThirdPerson/Blueprints/BP_ThirdPersonCharacter` (`GameplayStatics.GetPlayerPawn` 0)))
  (set `self.As BP Third Person Character` _asbp_third_person_character))

(event `self.ReceiveTick`
  (params (DeltaSeconds :type "Float (single-precision)")))

(event `self.plate.OnComponentBeginOverlap`
  (params (OverlappedComponent :type "PrimitiveComponent Object Reference") (OtherActor :type "Actor Object Reference") (OtherComp :type "PrimitiveComponent Object Reference") (OtherBodyIndex :type Integer) (bFromSweep :type Boolean) (SweepResult :type "HitResult Structure (by ref)"))
  (`/Engine/EditorBlueprintResources/StandardMacros.DoOnce` false
    (:`Completed`
      (`/Game/ThirdPerson/Blueprints/BP_ThirdPersonCharacter.damagespike` (`self.As BP Third Person Character`))
      (`SceneComponent.SetRelativeScale3D` (`self.spike1`) (1.0 1.0 1.0))
      (`SceneComponent.SetRelativeScale3D` (`self.spike`) (1.0 1.0 1.0))
      (`SceneComponent.SetRelativeScale3D` (`self.spike2`) (1.0 1.0 1.0))
      (`SceneComponent.SetRelativeScale3D` (`self.spike3`) (1.0 1.0 1.0))
      (`SceneComponent.SetRelativeScale3D` (`self.spike5`) (1.0 1.0 1.0))
      (`SceneComponent.SetRelativeScale3D` (`self.spike6`) (1.0 1.0 1.0))
      (`SceneComponent.SetRelativeScale3D` (`self.spike7`) (1.0 1.0 1.0))
      (`SceneComponent.SetRelativeScale3D` (`self.spike8`) (1.0 1.0 1.0))
      (`SceneComponent.SetRelativeScale3D` (`self.spike9`) (1.0 1.0 1.0))
      (`KismetSystemLibrary.Delay` 0.5)
      (`self.K2_DestroyActor`))))

(fn `UserConstructionScript`)